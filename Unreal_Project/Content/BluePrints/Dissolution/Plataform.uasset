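; Platform actor from the Dissolution folder that drives a burn-dissolve material parameter on its static mesh when P is pressed.
; BeginPlay creates a dynamic material instance from the mesh's first material and assigns it to that slot.
; Pressing P sets the AllowBurn scalar to zero and plays the DisolutionValue timeline.
; Each timeline update writes the same constant zero to AllowBurn, with no timeline output used.
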(event `self.ReceiveBeginPlay`
  (bind _returnvalue (`KismetMaterialLibrary.CreateDynamicMaterialInstance` (`|GetArrayItem` (`MeshComponent.GetMaterials` (`self.StaticMesh`)))))
  (`PrimitiveComponent.SetMaterial` (`self.StaticMesh`) 0 _returnvalue))

(event `Key|P`
  (params (Key :type "Key Structure"))
  (:`Pressed`
    (`MeshComponent.SetScalarParameterValueOnMaterials` (`self.StaticMesh`) "AllowBurn" 0.0)
    (`Timeline|DisolutionValue`
      (:`Update`
        (`MeshComponent.SetScalarParameterValueOnMaterials` (`self.StaticMesh`) "AllowBurn" 0.0)))))

(fn `UserConstructionScript`)