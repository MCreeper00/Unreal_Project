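; Puzzle door actor that slides vertically when told to open or close through the OPEN_DOOR and CLOSE_DOOR events.
; Those events set flags that Tick reads to move the actor along Z at a fixed speed, with opening taking priority.
; Both directions share a Delay that stops motion by clearing the flags and setting IsOpen.
; Movement only runs while IsOpen is false, and nothing here resets it.
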(event `self.ReceiveBeginPlay`
  (set `self.Opening` false)
  (set `self.Closing` false)
  (set `self.Speed` 100.0))

(event `OPEN_DOOR`
  (set `self.Opening` true))

(event `CLOSE_DOOR`
  (set `self.Closing` true))

(event `self.ReceiveTick`
  (params (DeltaSeconds :type "Float (single-precision)"))
  (bind _returnvalue (`self.GetTransform`))
  (bind _returnvalue_2 (* DeltaSeconds (`self.Speed`)))
  (if (`self.isOpen`)
    _
    (elif (`self.Opening`)
      (`self.K2_SetActorTransform` (`KismetMathLibrary.MakeTransform` (`KismetMathLibrary.MakeVector` (.x (.location _returnvalue)) (.y (.location _returnvalue)) (+ (.z (.location _returnvalue)) _returnvalue_2)) (.rotation _returnvalue) (.scale _returnvalue)))
      (`KismetSystemLibrary.Delay` 4.5 :!label _label)
      (set `self.Opening` false)
      (set `self.Closing` false)
      (set `self.isOpen` true)
      (elif (`self.Closing`)
        (`self.K2_SetActorTransform` (`KismetMathLibrary.MakeTransform` (`KismetMathLibrary.MakeVector` (.x (.location _returnvalue)) (.y (.location _returnvalue)) (- (.z (.location _returnvalue)) _returnvalue_2)) (.rotation _returnvalue) (.scale _returnvalue)))
        (goto _label)))))

(fn `UserConstructionScript`)