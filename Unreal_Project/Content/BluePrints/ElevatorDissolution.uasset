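; An elevator platform actor that moves up and down and burns away when the first-person character enters its trigger box.
; Tick shifts it vertically at constant speed, with a Delay inside Tick flipping direction about every three seconds.
; The overlap enables the material's burn parameter and plays a timeline that drives the dissolution value, then destroys the actor.
; A custom event, not called here, sets up a dynamic material instance.
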(event `CustomEvent`
  (bind _returnvalue (`KismetMaterialLibrary.CreateDynamicMaterialInstance` (`|GetArrayItem` (`MeshComponent.GetMaterials` (`self.StaticMeshComponent`)))))
  (`PrimitiveComponent.SetMaterial` (`self.StaticMeshComponent`) 0 _returnvalue))

(event `self.Box1.OnComponentBeginOverlap`
  (params (OverlappedComponent :type "PrimitiveComponent Object Reference") (OtherActor :type "Actor Object Reference") (OtherComp :type "PrimitiveComponent Object Reference") (OtherBodyIndex :type Integer) (bFromSweep :type Boolean) (SweepResult :type "HitResult Structure (by ref)"))
  (cast `/Game/Character/FirstPersonBP/Blueprints/FirstPersonCharacter` OtherActor)
  (`MeshComponent.SetScalarParameterValueOnMaterials` (`self.StaticMeshComponent`) "AllowBurn" 1.0)
  (bind (_direction _newtrack_0) (`Timeline|Timeline_0`)
    (:`Update`
      (`MeshComponent.SetScalarParameterValueOnMaterials` (`self.StaticMeshComponent`) "DissolutionVal" (/ _newtrack_0 4.0)))
    (:`Finished`
      (`self.K2_DestroyActor`))))

(event `self.ReceiveBeginPlay`
  (set `self.goingUp` true)
  (set `self.speed` 100.0))

(event `self.ReceiveTick`
  (params (DeltaSeconds :type "Float (single-precision)"))
  (bind _returnvalue (`self.GetTransform`))
  (bind _returnvalue_2 (* DeltaSeconds (`self.speed`)))
  (if (`self.goingUp`)
    (`self.K2_SetActorTransform` (`KismetMathLibrary.MakeTransform` (`KismetMathLibrary.MakeVector` (.x (.location _returnvalue)) (.y (.location _returnvalue)) (+ (.z (.location _returnvalue)) _returnvalue_2)) (.rotation _returnvalue) (.scale _returnvalue)))
    (else
      (`self.K2_SetActorTransform` (`KismetMathLibrary.MakeTransform` (`KismetMathLibrary.MakeVector` (.x (.location _returnvalue)) (.y (.location _returnvalue)) (- (.z (.location _returnvalue)) _returnvalue_2)) (.rotation _returnvalue) (.scale _returnvalue)))))
  (`KismetSystemLibrary.Delay` 3.0)
  (set `self.goingUp` (not (`self.goingUp`))))

(fn `UserConstructionScript`)