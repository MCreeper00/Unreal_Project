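; Door actor that slides vertically, rising on the OPEN_DOOR event and lowering on CLOSE_DOOR.
; Both events set flags that Tick reads to move the actor at a constant speed, with a fixed Delay clearing each flag to end the travel.
; CanOpen blocks rising during a close, and CancelNext swallows a following request when one arrives while both flags are set.
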(event `self.ReceiveBeginPlay`
  (set `self.Opening` false)
  (set `self.Closing` false)
  (set `self.Speed` 100.0)
  (set `self.CancelNext` false)
  (set `self.CanOpen` true))

(event `OPEN_DOOR`
  (if (`self.CancelNext`)
    (set `self.CancelNext` false)
    (else
      (if (and (`self.Opening`) (`self.Closing`))
        (set `self.CancelNext` true))
      (set `self.Opening` true))))

(event `CLOSE_DOOR`
  (if (`self.CancelNext`)
    (set `self.CancelNext` false)
    (else
      (if (and (`self.Opening`) (`self.Closing`))
        (set `self.CancelNext` true))
      (set `self.Closing` true))))

(event `self.ReceiveTick`
  (params (DeltaSeconds :type "Float (single-precision)"))
  (bind _returnvalue (`self.GetTransform`))
  (bind _returnvalue_2 (* DeltaSeconds (`self.Speed`)))
  (if (`self.Opening`)
    (if (`self.CanOpen`)
      (`self.K2_SetActorTransform` (`KismetMathLibrary.MakeTransform` (`KismetMathLibrary.MakeVector` (.x (.location _returnvalue)) (.y (.location _returnvalue)) (+ (.z (.location _returnvalue)) _returnvalue_2)) (.rotation _returnvalue) (.scale _returnvalue)))
      (`KismetSystemLibrary.Delay` 4.5)
      (set `self.Opening` false)
      (else
        (if (`self.Closing`) :!label _label
          (`self.K2_SetActorTransform` (`KismetMathLibrary.MakeTransform` (`KismetMathLibrary.MakeVector` (.x (.location _returnvalue)) (.y (.location _returnvalue)) (- (.z (.location _returnvalue)) _returnvalue_2)) (.rotation _returnvalue) (.scale _returnvalue)))
          (set `self.CanOpen` false)
          (`KismetSystemLibrary.Delay` 4.5)
          (set `self.Closing` false)
          (set `self.CanOpen` true))))
    (elif (not (`self.CancelNext`))
      (goto _label))))

(fn `UserConstructionScript`)