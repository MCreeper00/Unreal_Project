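; Elevator actor that moves continuously up and down along the world Z axis.
; BeginPlay sets the upward direction and speed, and Tick offsets the transform by speed times delta time, keeping rotation and scale.
; A Delay chained on Tick ignores calls while pending, so the direction flips about every three seconds, making travel time-based with no height limits.
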(event `self.ReceiveBeginPlay`
  (set `self.goingUp` true)
  (set `self.speed` 100.0))

(event `self.ReceiveTick`
  (params (DeltaSeconds :type "Float (single-precision)"))
  (bind _returnvalue (`self.GetTransform`))
  (bind _returnvalue_2 (* DeltaSeconds (`self.speed`)))
  (if (`self.goingUp`)
    (`self.K2_SetActorTransform` (`KismetMathLibrary.MakeTransform` (`KismetMathLibrary.MakeVector` (.x (.location _returnvalue)) (.y (.location _returnvalue)) (+ (.z (.location _returnvalue)) _returnvalue_2)) (.rotation _returnvalue) (.scale _returnvalue)))
    (else
      (`self.K2_SetActorTransform` (`KismetMathLibrary.MakeTransform` (`KismetMathLibrary.MakeVector` (.x (.location _returnvalue)) (.y (.location _returnvalue)) (- (.z (.location _returnvalue)) _returnvalue_2)) (.rotation _returnvalue) (.scale _returnvalue)))))
  (`KismetSystemLibrary.Delay` 3.0)
  (set `self.goingUp` (not (`self.goingUp`))))

(fn `UserConstructionScript`)